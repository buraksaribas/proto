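; Player controller for the multiplayer menu and lobby, with UI-only input for the local player.
; Creates lobby, character and loading screen widgets, blends the camera between pawn and lobby character view via authority checks and SR_ events, and can end client sessions.
; Loads and saves the player profile, including selected character, through SG_PlayerProfile.
; SR_ events pass profile, character and ready changes to GM_Menu, while update events refresh the lobby widget.
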(event `self.ReceiveBeginPlay`
  ;[1 1 1] beginplay
  (if (`self.IsLocalController`)
    (`WidgetBlueprintLibrary.SetInputMode_UIOnlyEx` self null)
    (set `self.bShowMouseCursor` true)))

(event `CreateLobbyMenu`
  ;[1 1 1] create lobby menu
  (bind _lobbymenuwb (`self.LobbyMenuWB`)
    (:`then`
      _)
    (:`else`
      (bind _returnvalue (`|CreateWidget` "/Game/Widgets/LobbyMenu/WB_LobbyMenu.WB_LobbyMenu_C" self))
      (set `self.LobbyMenuWB` _returnvalue)))
  (`UserWidget.AddToViewport` _lobbymenuwb 0)
  (`/Engine/EditorBlueprintResources/ActorMacros.Switch Has Authority`
    (:`Authority`
      (`self.SetViewTargetWithBlend` (`self.K2_GetPawn`) 1.0))
    (:`Remote`
      (`self.SR_SetViewTargetNormal`))))

(event `SR_SetViewTargetNormal`
  ;[1 1 1] create lobby menu
  ;;[1 1 1] SR - set view target to normal
  (`self.SetViewTargetWithBlend` (`self.K2_GetPawn`) 1.0))

(event `EndClientSession`
  ;[1 1 1] end client session
  (`DestroySessionCallbackProxy.DestroySession` self
    (:`OnSuccess`
      (`GameplayStatics.OpenLevel` "MainMenu_Map"))
    (:`OnFailure`
      (`KismetSystemLibrary.PrintString` "Failed to destroy session"))))

(event `CreateLoadingScreen`
  ;[1 1 1] create loading screen
  (bind _loadingscreenwb (`self.LoadingScreenWB`)
    (:`then`
      _)
    (:`else`
      (bind _returnvalue (`|CreateWidget` "/Game/Widgets/Common/WB_LoadingScreen.WB_LoadingScreen_C" self))
      (set `self.LoadingScreenWB` _returnvalue)))
  (`UserWidget.AddToViewport` _loadingscreenwb 0))

(event `InitialSetup`
  ;[1 1 1] initial setup
  (`self.LoadPlayerProfile`)
  (`self.SR_UpdateLobby` (`self.PlayerProfile`)))

(event `ShowCharacterMenu`
  ;[1 1 1] Show character menu
  (bind _charactermenuwb (`self.CharacterMenuWB`)
    (:`then`
      _)
    (:`else`
      (bind _returnvalue (`|CreateWidget` "/Game/Widgets/LobbyMenu/WB_CharacterMenu.WB_CharacterMenu_C" self))
      (set `self.CharacterMenuWB` _returnvalue)))
  (`UserWidget.AddToViewport` _charactermenuwb 0)
  (`/Engine/EditorBlueprintResources/ActorMacros.Switch Has Authority`
    (:`Authority`
      (`self.SetViewTargetWithBlend` (`ChildActorComponent.ChildActor` (`/Game/Blueprints/Gameplay/Lobby/BP_LobbyCharacter.ViewTarget` (`self.LobbyCharacterBP`))) 1.0))
    (:`Remote`
      (`self.SR_SetViewTargetCharacter`))))

(event `SR_UpdateLobby`
  (params (PlayerProfile :type "/Game/Blueprints/Common/S_PlayerProfile Structure"))
  ;[1 1 1] SR - update lobby
  (set `self.PlayerProfile` PlayerProfile)
  (bind _asgm_menu (cast `/Game/Blueprints/Framework/Menu/GM_Menu` (`GameplayStatics.GetGameMode`)))
  (`/Game/Blueprints/Framework/Menu/GM_Menu.UpdateLobby` _asgm_menu true true true true))

(event `SR_SetViewTargetCharacter`
  ;[1 1 1] Show character menu
  ;;[1 1 1] SR - set view target to character
  (`self.SetViewTargetWithBlend` (`ChildActorComponent.ChildActor` (`/Game/Blueprints/Gameplay/Lobby/BP_LobbyCharacter.ViewTarget` (`self.LobbyCharacterBP`))) 1.0))

(event `UpdatePlayerList`
  (params (PlayerProfiles :type "Array of /Game/Blueprints/Common/S_PlayerProfile Structure (by ref)"))
  ;[1 1 1] update player list
  (`/Game/Widgets/LobbyMenu/WB_LobbyMenu.UpdatePlayerNames` (`self.LobbyMenuWB`) PlayerProfiles))

(event `UpdateLevelSelection`
  (params (RowName :type Name))
  ;[1 1 1] update level selection
  (`/Game/Widgets/LobbyMenu/WB_LobbyMenu.UpdateLevelSelection` (`self.LobbyMenuWB`) RowName))

(event `SR_UpdatePlayerReady`
  (params (`Ready?` :type Boolean))
  (bind _asgm_menu (cast `/Game/Blueprints/Framework/Menu/GM_Menu` (`GameplayStatics.GetGameMode`)))
  (`/Game/Blueprints/Framework/Menu/GM_Menu.SetPlayerReady` _asgm_menu self `Ready?`))

(event `UpdatePlayerReady`
  (params (`PlayersReady?` :type "Array of Boolean"))
  (`/Game/Widgets/LobbyMenu/WB_LobbyMenu.UpdatePlayersReady` (`self.LobbyMenuWB`) `PlayersReady?`))

(event `SR_UpdateSelectedCharacter`
  (params (PlayerProfile :type "/Game/Blueprints/Common/S_PlayerProfile Structure"))
  ;[1 1 1] SR - update selected character
  (bind _output_get (set `self.PlayerProfile` PlayerProfile))
  (bind _asgm_menu (cast `/Game/Blueprints/Framework/Menu/GM_Menu` (`GameplayStatics.GetGameMode`)))
  (`/Game/Blueprints/Framework/Menu/GM_Menu.UpdateCharacterForController` _asgm_menu self _output_get))

(fn `LoadPlayerProfile`
  (locals (Lcl_PlayerProfileSlot :type String :default "PlayerProfileSlot"))
  (bind _returnvalue (`GameplayStatics.DoesSaveGameExist` (`local.Lcl_PlayerProfileSlot`)))
  (if (not _returnvalue)
    (bind _returnvalue_2 (`GameplayStatics.CreateSaveGameObject` "/Game/Blueprints/Common/SG_PlayerProfile.SG_PlayerProfile_C"))
    (`GameplayStatics.SaveGameToSlot` _returnvalue_2 (`local.Lcl_PlayerProfileSlot`)))
  (bind _returnvalue_3 (`GameplayStatics.LoadGameFromSlot` (`local.Lcl_PlayerProfileSlot`)))
  (bind _assg_player_profile (cast `/Game/Blueprints/Common/SG_PlayerProfile` _returnvalue_3))
  (set `self.PlayerProfile` (`/Game/Blueprints/Common/SG_PlayerProfile.PlayerProfile` _assg_player_profile)))

(fn `SaveSelectedCharacter`
  (params (CharacterRowName :type Name) (CharacterClass :type "Character Class Reference"))
  (bind _playerprofilesg (`self.PlayerProfileSG`))
  (setmembers `/Game/Blueprints/Common/S_PlayerProfile` :`StructRef` (`self.PlayerProfile`) :`CharacterRowName` CharacterRowName :`CharacterClass` CharacterClass)
  (`/Engine/EditorBlueprintResources/StandardMacros.IsValid` (`self.PlayerProfileSG`)
    (:`Is Valid`
      _)
    (:`Is Not Valid`
      (bind _returnvalue (`GameplayStatics.CreateSaveGameObject` "/Game/Blueprints/Common/SG_PlayerProfile.SG_PlayerProfile_C"))
      (set `self.PlayerProfileSG` _returnvalue)))
  (set `/Game/Blueprints/Common/SG_PlayerProfile.PlayerProfile` (`self.PlayerProfile`) _playerprofilesg)
  (`GameplayStatics.SaveGameToSlot` _playerprofilesg "PlayerProfileSlot")
  (`self.SR_UpdateSelectedCharacter` (`self.PlayerProfile`)))

(fn `UserConstructionScript`)