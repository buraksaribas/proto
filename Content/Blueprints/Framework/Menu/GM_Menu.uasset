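; Menu game mode that manages the multiplayer lobby: connected players, their profiles and their preview characters.
; On login to the lobby map it registers each menu controller and starts its lobby UI.
; Lobby updates copy profiles into player states, push player list and level choice to controllers, and refresh named characters with data table meshes on free spots.
; Logout destroys that player's character, frees the spot and refreshes the lobby.
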(event `self.K2_PostLogin`
  (params (NewPlayer :type "PlayerController Object Reference"))
  (bind _returnvalue (`GameplayStatics.GetCurrentLevelName` true))
  (switch `string` _returnvalue
    (:`LobbyMenu_Map`
      (bind _aspc_menu (cast `/Game/Blueprints/Framework/Menu/PC_Menu` NewPlayer))
      (`KismetArrayLibrary.Array_Add` (`self.All_ConnectedPlayers`) _aspc_menu)
      (`/Game/Blueprints/Framework/Menu/PC_Menu.CreateLobbyMenu` _aspc_menu)
      (`/Game/Blueprints/Framework/Menu/PC_Menu.InitialSetup` _aspc_menu))))

(event `UpdateLobby`
  (params (PlayerList :type Boolean) (LevelSelection :type Boolean) (CharacterSelection :type Boolean))
  (`KismetArrayLibrary.Array_Clear` (`self.All_PlayerProfiles`))
  (for (_array_element _array_index) (`self.All_ConnectedPlayers`)
    (bind _playerprofile (`/Game/Blueprints/Framework/Menu/PC_Menu.PlayerProfile` _array_element))
    (`KismetArrayLibrary.Array_Set` (`self.All_PlayerProfiles`) _array_index _playerprofile true)
    (bind _asps_game (cast `/Game/Blueprints/Framework/Common/PS_Game` (`Controller.PlayerState` _array_element)))
    (set `/Game/Blueprints/Framework/Common/PS_Game.PlayerProfile` _playerprofile _asps_game))
  (for (_array_element_2 _array_index_2) (`self.All_ConnectedPlayers`)
    (if PlayerList
      (`/Game/Blueprints/Framework/Menu/PC_Menu.UpdatePlayerList` _array_element_2 (`self.All_PlayerProfiles`)))
    (if LevelSelection
      (`/Game/Blueprints/Framework/Menu/PC_Menu.UpdateLevelSelection` _array_element_2 (`self.SelectedLevelName`)))
    (if CharacterSelection
      (`self.UpdateSelectedCharacter` _array_index_2))))

(event `self.K2_OnLogout`
  (params (ExitingController :type "Controller Object Reference"))
  (bind _aspc_menu (cast `/Game/Blueprints/Framework/Menu/PC_Menu` ExitingController))
  (bind _lobbycharacterbp (`/Game/Blueprints/Framework/Menu/PC_Menu.LobbyCharacterBP` _aspc_menu))
  (if (not (== _lobbycharacterbp null))
    (`self.K2_DestroyActor` _lobbycharacterbp)
    (set `/Game/Blueprints/Gameplay/Lobby/BP_LobbyPlayerSpot.SpotUsed?` false (`/Game/Blueprints/Framework/Menu/PC_Menu.LobbyPlayerSpotBP` _aspc_menu)))
  (`KismetArrayLibrary.Array_RemoveItem` (`self.All_ConnectedPlayers`) _aspc_menu)
  (`self.UpdateLobby` true false true))

(event `UpdateSelectedCharacter`
  (params (PlayerIndex :type Integer))
  (bind _output (`|GetArrayItem` (`self.All_ConnectedPlayers`) PlayerIndex))
  (bind (_playername _characterrowname) (break `/Game/Blueprints/Common/S_PlayerProfile` (`|GetArrayItem` (`self.All_PlayerProfiles`) PlayerIndex)))
  (bind _lobbycharacterbp (`/Game/Blueprints/Framework/Menu/PC_Menu.LobbyCharacterBP` _output))
  (if (== _lobbycharacterbp null)
    (bind _availableplayerspot (`self.GetLobbyPlayerSpot`))
    (set `/Game/Blueprints/Gameplay/Lobby/BP_LobbyPlayerSpot.SpotUsed?` true _availableplayerspot)
    (bind _returnvalue (`|SpawnActorFromClass` "/Game/Blueprints/Gameplay/Lobby/BP_LobbyCharacter.BP_LobbyCharacter_C" (`self.GetTransform` _availableplayerspot) "Undefined" "MultiplyWithRoot" null null))
    (set `/Game/Blueprints/Framework/Menu/PC_Menu.LobbyCharacterBP` _returnvalue _output)
    (set `/Game/Blueprints/Framework/Menu/PC_Menu.LobbyPlayerSpotBP` _availableplayerspot _output))
  (`/Game/Blueprints/Gameplay/Lobby/BP_LobbyCharacter.MC_SetPlayerName` _lobbycharacterbp _playername)
  (bind _returnvalue_2 (`|GetDataTableRow` "/Game/Data/DT_CharacterInfo.DT_CharacterInfo" _characterrowname)
    (:`then`
      (`/Game/Blueprints/Gameplay/Lobby/BP_LobbyCharacter.MC_SetCharacterMesh` _lobbycharacterbp (`.CharacterMesh_3_1D7A89644B7E1AC2789EEFA2E0D0B8A9` (break `/Game/Blueprints/Characters/S_CharacterInfo` _returnvalue_2))))))

(event `UpdateCharacterForController`
  (params (Controller :type "/Game/Blueprints/Framework/Menu/PC_Menu Object Reference") (PlayerProfile :type "/Game/Blueprints/Common/S_PlayerProfile Structure"))
  (bind _returnvalue (`KismetArrayLibrary.Array_Find` (`self.All_ConnectedPlayers`) Controller))
  (`KismetArrayLibrary.Array_Set` (`self.All_PlayerProfiles`) _returnvalue PlayerProfile true)
  (bind _asps_game (cast `/Game/Blueprints/Framework/Common/PS_Game` (`Controller.PlayerState` Controller)))
  (set `/Game/Blueprints/Framework/Common/PS_Game.PlayerProfile` PlayerProfile _asps_game)
  (`self.UpdateSelectedCharacter` _returnvalue))

(fn `GetLobbyPlayerSpot`
  (returns (AvailablePlayerSpot :type "/Game/Blueprints/Gameplay/Lobby/BP_LobbyPlayerSpot Object Reference"))
  (if (== (`KismetArrayLibrary.Array_Length` (`self.All_LobbyPlayerSpots`)) 0)
    (bind _outactors (`GameplayStatics.GetAllActorsOfClass` "/Game/Blueprints/Gameplay/Lobby/BP_LobbyPlayerSpot.BP_LobbyPlayerSpot_C"))
    (set `self.All_LobbyPlayerSpots` _outactors))
  (for _array_element (`self.All_LobbyPlayerSpots`)
    (if (not (`/Game/Blueprints/Gameplay/Lobby/BP_LobbyPlayerSpot.SpotUsed?` _array_element))
      (break)))
  (return _array_element))

(fn `UserConstructionScript`)