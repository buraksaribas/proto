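; Gameplay game mode that holds player spawning until everyone expected has joined, then spawns each player's chosen character.
; PostLogin tracks gameplay controllers and, once their count matches the game instance's connected-player count, waits briefly and restarts each at the PlayerStart named by its list index.
; SpawnDefaultPawnFor is overridden to spawn the character class from the controller's PlayerProfile.
; Logout removes the controller from the list.
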(event `self.K2_PostLogin`
  (params (NewPlayer :type "PlayerController Object Reference"))
  (bind _aspc_gameplay (cast `/Game/Blueprints/Framework/Gameplay/PC_Gameplay` NewPlayer))
  (`KismetArrayLibrary.Array_Add` (`self.All_ConnectedPlayers`) _aspc_gameplay)
  (bind _asgi_game (cast `/Game/Blueprints/Framework/Common/GI_Game` (`GameplayStatics.GetGameInstance`)))
  (set `self.NumExpectedPlayers` (`/Game/Blueprints/Framework/Common/GI_Game.NumConnectedPlayers` _asgi_game))
  (if (== (`self.NumExpectedPlayers`) (`KismetArrayLibrary.Array_Length` (`self.All_ConnectedPlayers`)))
    (`KismetSystemLibrary.Delay` 1.0)
    (for (_array_element _array_index) (`self.All_ConnectedPlayers`)
      (`self.RestartPlayerAtPlayerStart` _array_element (`self.K2_FindPlayerStart` _array_element (`KismetStringLibrary.Conv_IntToString` _array_index))))))

(event `self.K2_OnLogout`
  (params (ExitingController :type "Controller Object Reference"))
  (bind _aspc_gameplay (cast `/Game/Blueprints/Framework/Gameplay/PC_Gameplay` ExitingController))
  (`KismetArrayLibrary.Array_RemoveItem` (`self.All_ConnectedPlayers`) _aspc_gameplay))

(fn `SpawnDefaultPawnFor`
  (params (NewPlayer :type "Controller Object Reference") (StartSpot :type "Actor Object Reference"))
  (returns (ReturnValue :type "Pawn Object Reference"))
  (bind _aspc_gameplay (cast `/Game/Blueprints/Framework/Gameplay/PC_Gameplay` NewPlayer))
  (bind _returnvalue (`|SpawnActorFromClass` (`.CharacterClass_8_32ED42564F6F4BFB06025D8310B1A06F` (break `/Game/Blueprints/Common/S_PlayerProfile` (`/Game/Blueprints/Framework/Gameplay/PC_Gameplay.PlayerProfile` _aspc_gameplay))) (`self.GetTransform` StartSpot) "Undefined" "MultiplyWithRoot" null null))
  (return _returnvalue))

(fn `UserConstructionScript`)