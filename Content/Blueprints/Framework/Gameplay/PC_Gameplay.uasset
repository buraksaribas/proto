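; PC_Gameplay is the gameplay player controller that sets up the local player's HUD, input and profile, and handles leaving a session.
; On BeginPlay the local controller shows WB_GameHUD, switches to game-only input and loads the player profile from a save slot.
; The authority stores the profile directly, while a remote client passes it through SR_SetPlayerProfile.
; EndClientSession destroys the session and returns to the main menu on success.
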(event `SR_SetPlayerProfile`
  (params (PlayerProfile :type "/Game/Blueprints/Common/S_PlayerProfile Structure"))
  (set `self.PlayerProfile` PlayerProfile))

(event `self.ReceiveBeginPlay`
  (if (`self.IsLocalPlayerController`)
    (`self.ShowGameHUD`)
    (`WidgetBlueprintLibrary.SetInputMode_GameOnly` self)
    (set `self.bShowMouseCursor` false)
    (bind _returnvalue (`GameplayStatics.LoadGameFromSlot` "PlayerProfileSlot"))
    (bind _assg_player_profile (cast `/Game/Blueprints/Common/SG_PlayerProfile` _returnvalue))
    (`/Engine/EditorBlueprintResources/ActorMacros.Switch Has Authority`
      (:`Authority`
        (bind _playerprofile (`/Game/Blueprints/Common/SG_PlayerProfile.PlayerProfile` _assg_player_profile))
        (set `self.PlayerProfile` _playerprofile))
      (:`Remote`
        (`self.SR_SetPlayerProfile` _playerprofile)))))

(event `EndClientSession`
  ;[1 1 1] end client session
  (`DestroySessionCallbackProxy.DestroySession` self
    (:`OnSuccess`
      (`GameplayStatics.OpenLevel` "MainMenu_Map"))
    (:`OnFailure`
      (`KismetSystemLibrary.PrintString` "Failed to destroy session"))))

(event `ShowGameHUD`
  ;[1 1 1] show game HUD
  (bind _gamehudwb (`self.GameHUDWB`)
    (:`then`
      _)
    (:`else`
      (bind _returnvalue (`|CreateWidget` "/Game/Widgets/Gameplay/WB_GameHUD.WB_GameHUD_C" self))
      (set `self.GameHUDWB` _returnvalue)))
  (`UserWidget.AddToViewport` _gamehudwb 0))

(fn `UserConstructionScript`)